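; BP_DDoor is an automatic double sliding door that opens when BP_FirstPersonCharacter enters its Box trigger and closes when it leaves.
; Overlap events play or reverse the DoorTimer timeline, whose alpha lerps Door1 and Door2 apart in opposite directions along local X.
; During timeline updates, each panel plays its own sound through a DoOnce with a delayed reset, using the relative offset as world location.
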(event OnComponentBeginOverlap(Box)
  (params (OverlappedComponent :type Primitive%20Component%20Object%20Reference) (OtherActor :type Actor%20Object%20Reference) (OtherComp :type Primitive%20Component%20Object%20Reference) (OtherBodyIndex :type Integer) (bFromSweep :type Boolean) (SweepResult :type Hit%20Result%20Structure%20%28by%20ref%29))
  (Utilities|Casting|CastToBP_FirstPersonCharacter OtherActor)
  (bind _float_alpha (Timeline|DoorTimer Play)
    (:Update
      (Utilities|FlowControl|Sequence
        (:then_0
          (Transformation|SetRelativeLocation (Variables|Default|GetDoor_1) (Math|Vector|Lerp(Vector) "0, 0,-31.037655" "60.000000, 0,-31.037655" _float_alpha) false false)
          (Utilities|FlowControl|DoOnce false :!label _label
            (:Completed
              (Audio|PlaySoundatLocation "/Game/Audio/New_Recording_7.New_Recording_7" (Math|Vector|Lerp(Vector) "0, 0,-31.037655" "60.000000, 0,-31.037655" _float_alpha) "0, 0, 0" 1.0 1.0 0.0 0 0 0 0)
              (Utilities|FlowControl|Delay 1.0)
              (goto _label Reset))))
        (:then_1
          (Transformation|SetRelativeLocation (Variables|Default|GetDoor_2) (Math|Vector|Lerp(Vector) "0.000000, 0,-31.037655" "-60.000000,0.000000,-31.037655" _float_alpha) false false)
          (Utilities|FlowControl|DoOnce false :!label _label_2
            (:Completed
              (Audio|PlaySoundatLocation "/Game/Audio/New_Recording_7_copy.New_Recording_7_copy" (Math|Vector|Lerp(Vector) "0.000000, 0,-31.037655" "-60.000000,0.000000,-31.037655" _float_alpha) "0, 0, 0" 1.0 1.0 0.0 0 0 0 0)
              (Utilities|FlowControl|Delay 1.0)
              (goto _label_2 Reset))))))))

(event OnComponentEndOverlap(Box)
  (params (OverlappedComponent :type Primitive%20Component%20Object%20Reference) (OtherActor :type Actor%20Object%20Reference) (OtherComp :type Primitive%20Component%20Object%20Reference) (OtherBodyIndex :type Integer))
  (Utilities|Casting|CastToBP_FirstPersonCharacter OtherActor)
  (bind _float_alpha (Timeline|DoorTimer Reverse)
    (:Update
      (Utilities|FlowControl|Sequence
        (:then_0
          (Transformation|SetRelativeLocation (Variables|Default|GetDoor_1) (Math|Vector|Lerp(Vector) "0, 0,-31.037655" "60.000000, 0,-31.037655" _float_alpha) false false)
          (Utilities|FlowControl|DoOnce false :!label _label
            (:Completed
              (Audio|PlaySoundatLocation "/Game/Audio/New_Recording_7.New_Recording_7" (Math|Vector|Lerp(Vector) "0, 0,-31.037655" "60.000000, 0,-31.037655" _float_alpha) "0, 0, 0" 1.0 1.0 0.0 0 0 0 0)
              (Utilities|FlowControl|Delay 1.0)
              (goto _label Reset))))
        (:then_1
          (Transformation|SetRelativeLocation (Variables|Default|GetDoor_2) (Math|Vector|Lerp(Vector) "0.000000, 0,-31.037655" "-60.000000,0.000000,-31.037655" _float_alpha) false false)
          (Utilities|FlowControl|DoOnce false :!label _label_2
            (:Completed
              (Audio|PlaySoundatLocation "/Game/Audio/New_Recording_7_copy.New_Recording_7_copy" (Math|Vector|Lerp(Vector) "0.000000, 0,-31.037655" "-60.000000,0.000000,-31.037655" _float_alpha) "0, 0, 0" 1.0 1.0 0.0 0 0 0 0)
              (Utilities|FlowControl|Delay 1.0)
              (goto _label_2 Reset))))))))

(fn ConstructionScript)